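; Stone-board puzzle actor that triggers a target's interaction when the correct combination of stones is selected.
; The construction script builds a stone grid sized by Rows and Columns, and BeginPlay maps CorrectCombination coordinates to the matching components.
; Overlapping the board's box switches to its camera with mouse clicking and an optional tutorial widget.
; Clicks highlight a capped set of stones, which the button checks regardless of order, with color and sound feedback.
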(event `self.ColBoxBoard.OnComponentBeginOverlap`
  (params (OverlappedComponent :type "PrimitiveComponent Object Reference") (OtherActor :type "Actor Object Reference") (OtherComp :type "PrimitiveComponent Object Reference") (OtherBodyIndex :type Integer) (bFromSweep :type Boolean) (SweepResult :type "HitResult Structure (by ref)"))
  (bind _returnvalue (`GameplayStatics.GetPlayerController` 0))
  (bind _returnvalue_2 (`GameplayStatics.GetPlayerController` 0))
  ;[1 1 1] Change View Stone Camera
  (if bFromSweep
    (`PlayerController.SetViewTargetWithBlend` _returnvalue self 1.0 "VTBlend_Linear" 0.0 false)
    (`WidgetBlueprintLibrary.SetInputMode_GameAndUIEx` _returnvalue null)
    (set `PlayerController.bShowMouseCursor` true _returnvalue_2)
    (set `PlayerController.bEnableClickEvents` true _returnvalue_2)
    (if (`self.IsTutorial`)
      (bind _returnvalue_3 (`|CreateWidget` "/Game/BluePrint/Tutorial/BluePrints/NewWidgetBlueprint.NewWidgetBlueprint_C" (`GameplayStatics.GetPlayerController` 0)))
      (`UserWidget.AddToViewport` _returnvalue_3 0)
      (if (`self.UIONLY`)
        (`WidgetBlueprintLibrary.SetInputMode_UIOnlyEx` (`GameplayStatics.GetPlayerController` 0) null)
        (set `self.UIONLY` false)))))

(event `self.ColBoxBoard.OnComponentEndOverlap`
  (params (OverlappedComponent :type "PrimitiveComponent Object Reference") (OtherActor :type "Actor Object Reference") (OtherComp :type "PrimitiveComponent Object Reference") (OtherBodyIndex :type Integer))
  (bind _returnvalue (`GameplayStatics.GetPlayerController` 0))
  ;[1 1 1] Change View Stone Camera
  (bind _asbp_third_person_character (cast `/Game/ThirdPerson/Blueprints/BP_ThirdPersonCharacter` OtherActor))
  (`PlayerController.SetViewTargetWithBlend` (`GameplayStatics.GetPlayerController` 0) _asbp_third_person_character 0.5 "VTBlend_Linear" 0.0 false)
  (`WidgetBlueprintLibrary.SetInputMode_GameOnly` _returnvalue)
  (set `PlayerController.bShowMouseCursor` false _returnvalue)
  (set `PlayerController.bEnableClickEvents` false _returnvalue)
  (set `self.IsTutorial` false))

(event `self.ReceiveBeginPlay`
  (bind _columns (`self.Columns`))
  ;[1 1 1] Stone Generation
  (for (_array_element _array_index) (`self.All buttons`)
    (add `PrimitiveComponent.OnClicked` _array_element (delegate `ClickComponent`))
    (if (`BlueprintSetLibrary.Set_Contains` (`self.Correct combination`) (make `/Game/BluePrint/StoneGeneration/S_pos` (mod _array_index _columns) (/ _array_index _columns)))
      (`BlueprintSetLibrary.Set_Add` (`self.Correct components`) _array_element)))
  (add `PrimitiveComponent.OnClicked` (`self.Button`) (delegate `ClickCheckButton`)))

(event `ClickComponent`
  (params (TouchedComponent :type "PrimitiveComponent Object Reference") (ButtonPressed :type "Key Structure" :default "None"))
  (bind _selected (`self.selected`))
  (bind _cheker (`self.Cheker`))
  (bind _returnvalue (`BlueprintSetLibrary.Set_Length` _selected))
  ;[1 1 1] StoneVerification
  (if (< (`self.Cheker`) 3)
    (if (not (`self.is open`))
      (`PrimitiveComponent.SetMaterial` TouchedComponent 0 "/Game/LevelObject/Materials/NeonMaterialInstance.NeonMaterialInstance")
      (`BlueprintSetLibrary.Set_Add` _selected TouchedComponent)
      (if (and (== _returnvalue 1) (== _cheker 1))
        _
        (elif (not (and (== _returnvalue 2) (== _cheker 2)))
          (`/Engine/EditorBlueprintResources/StandardMacros.IncrementInt` (`self.Cheker`)))))))

(event `ClickCheckButton`
  (params (TouchedComponent :type "PrimitiveComponent Object Reference") (ButtonPressed :type "Key Structure" :default "None"))
  (bind _target (`self.target`))
  (bind _selected (`self.selected`))
  ;[1 1 1] StoneVerification
  (if (not (`self.is open`))
    (bind _result (`BlueprintSetLibrary.Set_ToArray` _selected))
    (for _array_element _result
      (bind _asprimitive_component (cast `PrimitiveComponent` _array_element))
      (`PrimitiveComponent.SetMaterial` _asprimitive_component 0 "/Game/LevelObject/Materials/StoneMaterial.StoneMaterial")
      (set `self.Cheker` 0))
    (if (== (`BlueprintSetLibrary.Set_Length` _selected) (`BlueprintSetLibrary.Set_Length` (`self.Correct Components`)))
      (bind _result_2 (`BlueprintSetLibrary.Set_ToArray` _selected))
      (for _array_element_2 _result_2
        (if (not (`BlueprintSetLibrary.Set_Contains` (`self.Correct Components`) _array_element_2))
          (`BlueprintSetLibrary.Set_Clear` (`self.selected`))
          (set `self.is correct` false)
          (break)))
      (if (`self.is correct`)
        (set `self.is open` true)
        (`/Engine/EditorBlueprintResources/StandardMacros.IsValid` _target
          (:`Is Valid`
            (message `/Game/BluePrint/Interact/I_INTERACT.Interact` _target)
            (`PrimitiveComponent.SetMaterial` TouchedComponent 0 "/Game/BluePrint/StonePuzzle2/MESHES/Material_001.Material_001")
            (bind _returnvalue (`GameplayStatics.CreateSound2D` "/Game/BluePrint/StoneGeneration/yes.yes" 1.0 1.0 0.0 null))
            (`AudioComponent.Play` _returnvalue 0.0)
            (`KismetSystemLibrary.Delay` 0.2)
            (`PrimitiveComponent.SetMaterial` TouchedComponent 0 "/Game/Gang_Male_Sport/Material/Normal/M_Floor.M_Floor")))
        (else
          (set `self.is correct` true)
          (`PrimitiveComponent.SetMaterial` TouchedComponent 0 "/Game/BluePrint/StonePuzzle2/MESHES/Material_004.Material_004")
          (bind _returnvalue_2 (`GameplayStatics.CreateSound2D` "/Game/BluePrint/StoneGeneration/no.no" 1.0 1.0 0.0 null))
          (`AudioComponent.Play` _returnvalue_2 0.0)
          (`KismetSystemLibrary.Delay` 0.2)
          (`PrimitiveComponent.SetMaterial` TouchedComponent 0 "/Game/Gang_Male_Sport/Material/Normal/M_Floor.M_Floor")))
      (else
        (`BlueprintSetLibrary.Set_Clear` (`self.selected`))))
    (else
      (set `self.Cheker` 0))))

(fn `UserConstructionScript`
  (locals (thickness :type "Float (double-precision)" :default 4.0))
  (bind _board (`self.Board`))
  (`|ExecutionSequence`
    (:`then_0`
      (for _index (range (`self.Rows`))
        (for _index_2 (range (+ (- (`self.Columns`) 1 0) 1))
          (bind _returnvalue (`AddComponent|NODE_AddStaticMeshComponent-0` :`RelativeTransform` (`KismetMathLibrary.MakeTransform` (+ (`KismetMathLibrary.MakeVector` (`KismetMathLibrary.Conv_IntToDouble` (* _index_2 100)) 0.0 (`KismetMathLibrary.Conv_IntToDouble` (* _index -90))) (`KismetMathLibrary.MakeVector` (/ (* (`KismetMathLibrary.Conv_IntToDouble` (- (`self.Columns`) 1)) 100.0) -2.0) 0.0 (/ (* (`KismetMathLibrary.Conv_IntToDouble` (- (`self.Rows`) 1)) -90.0) -2.0))) (struct) (0.3 0.3 0.3))))
          (`KismetArrayLibrary.Array_Add` (`self.All buttons`) _returnvalue)
          (`SceneComponent.K2_SetRelativeLocation` (`self.Rune1`) (0.0 0.0 0.0) false false))))
    (:`then_1`
      (`SceneComponent.K2_SetRelativeLocation` (`self.Button`) (`KismetMathLibrary.MakeVector` 0.0 30.0 (* (`self.Rows`) -60.0)) false false))
    (:`then_2`
      (`SceneComponent.SetWorldScale3D` _board (`KismetMathLibrary.MakeVector` (* (`self.Columns`) 1.0) (/ (* (`local.thickness`) 0.5) 4.0) (* (`self.Rows`) 1.0)))
      (`SceneComponent.K2_SetRelativeLocation` _board (0.0 -25.0 0.0) false false))
    (:`then_3`
      (`SceneComponent.K2_AddRelativeLocation` (`self.Rune1`) (-280.0 -3e-06 -90.0) false false)
      (`SceneComponent.K2_AddRelativeLocation` (`self.number1`) (0.0 0.0 0.0) false false))))